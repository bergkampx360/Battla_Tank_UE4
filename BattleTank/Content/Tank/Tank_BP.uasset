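; Player-drivable tank pawn Blueprint that wires its aiming and movement components and maps player input to them.
; On BeginPlay it hands the barrel and turret to TankAiming and both tracks to TankMovement.
; Aim axes rotate an azimuth gimbal and spring arm scaled by delta time, while drive axes and Fire forward intents to the components.
; A reset action zeroes the tank's rotation and physics velocities.
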(event EventBeginPlay
  (Class|TankAimingComponent|Initialize (Variables|Default|GetTankAiming) (Variables|Default|GetBarrel) (Variables|Default|GetTankTurret))
  (Class|TankMovementComponent|Initialize (Variables|Default|GetTankMovement) (Variables|Default|GetLeftTrack) (Variables|Default|GetRightTrack)))

(event Input|ActionEvents|InputActionFire
  (params (Key :type Key%20Structure :default "AnyKey"))
  ;[1 1 1] Aiming, Firing Input Binding
  (:Pressed
    (Class|TankAimingComponent|Fire (Variables|Default|GetTankAiming))))

(event Input|ActionEvents|InputActionResetTank
  (params (Key :type Key%20Structure :default "AnyKey"))
  (bind _tank (Variables|Default|GetTank))
  ;[1 1 1] Reset tank rotation, velocity
  (:Pressed
    (Transformation|SetActorRotation self)
    (Physics|SetPhysicsLinearVelocity _tank "0, 0, 0" false "None")
    (Class|PrimitiveComponent|SetPhysicsAngularVelocity _tank "0, 0, 0" false "None")))

(event Input|AxisEvents|InputAxisAimAzimuth
  (params (AxisValue :type Float%20%28single-precision%29))
  ;[1 1 1] Aiming, Firing Input Binding
  (Transformation|AddLocalRotation (Variables|Default|GetAzimuth%20Gimbal) (Math|Rotator|MakeRotator 0.0 0.0 (* AxisValue (Utilities|Time|GetWorldDeltaSeconds) 1e+02)) false false))

(event Input|AxisEvents|InputAxisAimElevation
  (params (AxisValue :type Float%20%28single-precision%29))
  ;[1 1 1] Aiming, Firing Input Binding
  (Transformation|AddLocalRotation (Variables|Default|GetSpringArm) (Math|Rotator|MakeRotator 0.0 (* AxisValue (Utilities|Time|GetWorldDeltaSeconds) 1e+02) 0.0) false false))

(event Input|AxisEvents|InputAxisTurnRight
  (params (AxisValue :type Float%20%28single-precision%29))
  ;[1 1 1] Movement Input Binding
  (Class|TankMovementComponent|IntendTurnRight (Variables|Default|GetTankMovement) AxisValue))

(event Input|AxisEvents|InputAxisMoveForwardTrigger
  (params (AxisValue :type Float%20%28single-precision%29))
  ;[1 1 1] Movement Input Binding
  (Class|TankMovementComponent|IntendMoveForward (Variables|Default|GetTankMovement) AxisValue))

(event Input|AxisEvents|InputAxisMoveBackwardTrigger
  (params (AxisValue :type Float%20%28single-precision%29))
  ;[1 1 1] Movement Input Binding
  (Class|TankMovementComponent|IntendMoveForward (Variables|Default|GetTankMovement) AxisValue))

(fn ConstructionScript)